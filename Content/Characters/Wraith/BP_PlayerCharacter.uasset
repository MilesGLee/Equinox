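; Player character Blueprint for the Wraith, which can dive into a shadow movement mode while light detection allows it.
; In shadow mode, camera-relative line traces find a target point and surface orientation, wrapping around edges and rejecting NoWalk actors.
; Tick steers toward that target and ends shadow mode when diving is disallowed.
; It also reports noise outside shadow mode and handles interaction, pausing, saving, and death with fade-out and reload.
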(event `self.ReceiveBeginPlay`
  (set `self.target location` (`self.K2_GetActorLocation`))
  (`KismetSystemLibrary.K2_SetTimerDelegate` (`|CreateDelegate` :!event `Trace`) 0.2 true)
  (`KismetSystemLibrary.Delay` 0.2)
  (bind _asgm_bp_manager (cast `/Game/GameManager/GM_BP_Manager` (`GameplayStatics.GetGameMode`)))
  (`/Game/GameManager/GM_BP_Manager.Save Game` _asgm_bp_manager))

(event `InputAxis|Horizontal`
  (params (AxisValue :type "Float (single-precision)"))
  ;[1 1 1] Input Controles
  (set `self.HorizontalInput` AxisValue)
  (if (not (`self._inShadowMovement`)) :!label _label
    (`AISense_Hearing.ReportNoiseEvent` (`self.K2_GetActorLocation`) 50.0 self 30.0 "NotInShadowMode")))

(event `InputAxis|Vertical`
  (params (AxisValue :type "Float (single-precision)"))
  ;[1 1 1] Input Controles
  (set `self.VerticalInput` AxisValue)
  (goto _label))

(event `InputAction|Interact`
  (params (Key :type "Key Structure"))
  ;[1 1 1] Input Controles
  (:`Pressed`
    (`self.Interact`)))

(event `self.ReceiveTick`
  (params (DeltaSeconds :type "Float (single-precision)"))
  (`self.SetInput` (`self.HorizontalInput`) (`self.VerticalInput`))
  (`self.Move`)
  (if (`LightDetectionComponent.m_canDive` (`self.LightDetection`))
    _
    (elif (`self._inShadowMovement`)
      (`self.SetMovement` false)
      (if (not (`LightDetectionComponent.m_canDive` (`self.LightDetection`)))
        (set `self.IsDiving` false)))))

(event `InputAction|Shadow`
  (params (Key :type "Key Structure"))
  (bind (_returnvalue_x _returnvalue_y _returnvalue_z) (`KismetMathLibrary.BreakVector` (`self.GetVelocity`)))
  ;[1 1 1] Input Controles
  (:`Pressed`
    (if (`LightDetectionComponent.m_canDive` (`self.LightDetection`))
      (if (> _returnvalue_z -0.1)
        (`self.SwitchMovement`)
        (set `self.IsDiving` (`self._inShadowMovement`))))))

(event `Trace`
  (if (`self._inShadowMovement`)
    (`self.TraceMovement`)))

(event `Save Game`
  (bind _asgm_bp_manager (cast `/Game/GameManager/GM_BP_Manager` (`GameplayStatics.GetGameMode`)))
  (bind _output_get (set `self.As GM BP Manager` _asgm_bp_manager))
  (`/Game/GameManager/GM_BP_Manager.Save Game` _output_get))

(event `Move`
  (bind _returnvalue (`self.K2_GetActorLocation`))
  (bind _target_location (`self.target location`))
  (if (`self._inShadowMovement`)
    (if (> (+ (`KismetMathLibrary.Abs` (`self.VerticalInput`)) (`KismetMathLibrary.Abs` (`self.HorizontalInput`))) 0.0)
      (if (> (`KismetMathLibrary.Vector_Distance` _target_location _returnvalue) 2.0)
        (`self.AddMovementInput` (`KismetMathLibrary.GetDirectionUnitVector` _returnvalue _target_location))
        (`self.K2_SetActorRotation` (`KismetMathLibrary.RLerp` (`self.K2_GetActorRotation`) (`self.target rotation`) 0.01 true))))))

(event `OnDeath`
  (`CharacterMovementComponent.DisableMovement` (`self.CharacterMovement`))
  (`KismetSystemLibrary.Delay` 0.2)
  (bind _asgame_hud_bp (cast `/Game/UI/HUD_BP_GameHUD` (`PlayerController.GetHUD` (`GameplayStatics.GetPlayerController` 0))))
  (`/Game/UI/UW_BP_UserInterface.FadeToBlack` (`/Game/UI/HUD_BP_GameHUD.UI Ref` _asgame_hud_bp) "Forward" 0.3)
  (`/Game/GameManager/GM_BP_Manager.Load Game` (`self.As GM BP Manager`)))

(event `InputAction|Pause`
  (params (Key :type "Key Structure"))
  (bind _openmenu (`self.OpenMenu`))
  (:`Pressed`
    (bind _output_get (set `self.OpenMenu` (not (stale _output_get))))
    (if _openmenu
      (`GameplayStatics.SetGamePaused` _openmenu)
      (bind _returnvalue (`|CreateWidget` "/Game/UI/Pause_UW_BP.Pause_UW_BP_C" (`GameplayStatics.GetPlayerController` 0)))
      (`UserWidget.AddToViewport` _returnvalue 0)
      (else
        (`GameplayStatics.SetGamePaused` _openmenu)))))

(fn `GetMyMovementDirection`
  (returns (ReturnValue :type "Vector Structure"))
  (bind (_returnvalue_x _returnvalue_y _returnvalue_z) (`KismetMathLibrary.BreakVector` (`self.GetActorForwardVector`)))
  (bind (_returnvalue_x_2 _returnvalue_y_2 _returnvalue_z_2) (`KismetMathLibrary.BreakVector` (`self.GetActorRightVector`)))
  (bind (_returnvalue_x_3 _returnvalue_y_3) (`KismetMathLibrary.BreakVector` (`self.GetActorRightVector` (`self.PlayerCamera`))))
  (bind (_returnvalue_x_4 _returnvalue_y_4) (`KismetMathLibrary.BreakVector` (`self.GetActorForwardVector` (`self.PlayerCamera`))))
  (return (`KismetMathLibrary.Normal` (+ (* (`KismetMathLibrary.MakeVector` _returnvalue_x_4 _returnvalue_y_4 _returnvalue_z) (`self.VerticalInput`)) (* (`KismetMathLibrary.MakeVector` _returnvalue_x_3 _returnvalue_y_3 _returnvalue_z_2) (`self.HorizontalInput`))))))

(fn `TraceMovement`
  (locals (`hit F1` :type "HitResult Structure") (`hit F2` :type "HitResult Structure") (`hit R` :type "HitResult Structure"))
  (bind _returnvalue (`self.K2_GetActorLocation`))
  (bind _returnvalue_2 (`self.K2_GetActorLocation`))
  (bind _returnvalue_3 (`self.GetMyMovementDirection`))
  (bind _returnvalue_4 (`self.GetActorUpVector`))
  (bind _returnvalue_5 (`self.K2_GetActorLocation`))
  (bind (_hit_f1_bblockinghit _hit_f1_binitialoverlap _hit_f1_time _hit_f1_distance _hit_f1_location _hit_f1_impactpoint _hit_f1_normal _hit_f1_impactnormal _hit_f1_physmat _hit_f1_hitactor) (`GameplayStatics.BreakHitResult` (`local.hit F1`)))
  (bind (_hit_f1_bblockinghit_2 _hit_f1_binitialoverlap_2 _hit_f1_time_2 _hit_f1_distance_2 _hit_f1_location_2 _hit_f1_impactpoint_2 _hit_f1_normal_2 _hit_f1_impactnormal_2 _hit_f1_physmat_2 _hit_f1_hitactor_2) (`GameplayStatics.BreakHitResult` (`local.hit F1`)))
  (bind (_hit_f1_bblockinghit_3 _hit_f1_binitialoverlap_3 _hit_f1_time_3 _hit_f1_distance_3 _hit_f1_location_3 _hit_f1_impactpoint_3 _hit_f1_normal_3) (`GameplayStatics.BreakHitResult` (`local.hit F1`)))
  (bind (_hit_f2_bblockinghit _hit_f2_binitialoverlap _hit_f2_time _hit_f2_distance _hit_f2_location) (`GameplayStatics.BreakHitResult` (`local.hit F2`)))
  (bind (_hit_r_bblockinghit _hit_r_binitialoverlap _hit_r_time _hit_r_distance _hit_r_location) (`GameplayStatics.BreakHitResult` (`local.hit R`)))
  (bind _returnvalue_6 (`KismetMathLibrary.Normal` (+ (* (`self.GetMyMovementDirection`) 600.0) (* (`self.GetActorUpVector`) -500.0))))
  (bind _returnvalue_7 (`KismetMathLibrary.RotateAngleAxis` _returnvalue_6 90.0 (`self.GetActorRightVector`)))
  (bind _returnvalue_8 (+ (`self.K2_GetActorLocation`) (* _returnvalue_6 100.0)))
  (bind (_outhit _returnvalue_9) (`KismetSystemLibrary.LineTraceSingle` _returnvalue_5 (+ _returnvalue_5 (* _returnvalue_6 200.0)) "TraceTypeQuery1"))
  (if _returnvalue_9
    (set `local.hit F1` _outhit)
    (if (not (`self.ActorHasTag` _hit_f1_hitactor_2 "NoWalk"))
      (bind (_outhit_2 _returnvalue_10) (`KismetSystemLibrary.LineTraceSingle` _returnvalue (+ _returnvalue (* (`KismetMathLibrary.Normal` (+ (* (`self.GetMyMovementDirection`) 700.0) (* (`self.GetActorUpVector`) -500.0))) 200.0)) "TraceTypeQuery1"))
      (if _returnvalue_10
        (set `local.hit F2` _outhit_2)
        (bind (_outhit_3 _returnvalue_11) (`KismetSystemLibrary.LineTraceSingle` _returnvalue_2 (+ _returnvalue_2 (* _returnvalue_3 1000.0) (* _returnvalue_4 -500.0) (* (`KismetMathLibrary.RotateAngleAxis` _returnvalue_3 90.0 _returnvalue_4) 100.0)) "TraceTypeQuery1"))
        (if _returnvalue_11
          (set `local.hit R` _outhit_3)
          (set `self.target location` (+ _hit_f1_location_3 (* _hit_f1_normal_3 60.0)) :!label _label)
          (set `self.target rotation` (`KismetMathLibrary.MakeRotationFromAxes` (`KismetMathLibrary.GetDirectionUnitVector` _hit_f1_location_3 _hit_f2_location) (`KismetMathLibrary.GetDirectionUnitVector` _hit_f1_location_3 _hit_r_location) _hit_f1_normal_3)))
        (else
          (bind (_outhit_4 _returnvalue_12) (`KismetSystemLibrary.LineTraceSingle` _returnvalue_8 (+ _returnvalue_8 (* _returnvalue_7 200.0)) "TraceTypeQuery1" :!label _label_2))
          (if _returnvalue_12
            (set `local.hit F1` _outhit_4)
            (if (not (`self.ActorHasTag` _hit_f1_hitactor "NoWalk"))
              (bind (_outhit_5 _returnvalue_13) (`KismetSystemLibrary.LineTraceSingle` _returnvalue_8 (+ _returnvalue_8 (* (`KismetMathLibrary.RotateAngleAxis` _returnvalue_6 85.0 (`self.GetActorRightVector`)) 200.0)) "TraceTypeQuery1"))
              (if _returnvalue_13
                (set `local.hit F2` _outhit_5)
                (bind (_outhit_6 _returnvalue_14) (`KismetSystemLibrary.LineTraceSingle` _returnvalue_8 (+ _returnvalue_8 (* (`KismetMathLibrary.RotateAngleAxis` _returnvalue_7 5.0 _returnvalue_6) 200.0)) "TraceTypeQuery1"))
                (if _returnvalue_14
                  (set `local.hit R` _outhit_6)
                  (goto _label))))))))
    (else
      (goto _label_2))))

(fn `UserConstructionScript`)