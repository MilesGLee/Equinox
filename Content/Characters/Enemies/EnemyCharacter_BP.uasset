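; Enemy character that detects the player through AI perception and grabs them on contact.
; After a one-second delay, sight or velocity-gated hearing sets the HasSeenPlayer blackboard key and plays random step sounds, with hearing adding a growl.
; A retriggerable delay later clears detection and stops the audio.
; Player overlap with the box triggers a move to it, then freezes and turns the player, plays paired grab montages and loads the game.
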(event `self.ReceiveBeginPlay`
  (bind _returnvalue (`GameplayStatics.CreateSound2D` "/Game/Sounds/TwoSteping01.TwoSteping01" 0.1 1.0 0.0 null true false))
  (set `self.JoggerSound_1` _returnvalue)
  (bind _returnvalue_2 (`GameplayStatics.CreateSound2D` "/Game/Sounds/TwoStep2.TwoStep2" 0.1 1.0 0.0 null true false))
  (set `self.JoggerSound_2` _returnvalue_2)
  (bind _returnvalue_3 (`GameplayStatics.CreateSound2D` "/Game/Sounds/Step3.Step3" 0.1 1.0 0.0 null true false))
  (set `self.JoggerSound_3` _returnvalue_3)
  (bind _returnvalue_4 (`GameplayStatics.CreateSound2D` "/Game/Sounds/Grown.Grown" 0.1 1.0 0.0 null true false))
  (set `self.JoggerSound_4` _returnvalue_4))

(event `self.AIPerception.OnTargetPerceptionUpdated`
  (params (Actor :type "Actor Object Reference") (Stimulus :type "AIStimulus Structure"))
  (`KismetSystemLibrary.Delay` 1.0)
  (`|ExecutionSequence`
    (:`then_0`
      (`self.HandlesHearing` Actor Stimulus))
    (:`then_1`
      (`self.HandlesSight` Actor Stimulus)))
  (`KismetSystemLibrary.RetriggerableDelay` (`self.Duration`))
  (set `self.CoughtPlayer?` false)
  (`BlackboardComponent.SetValueAsBool` (`AIBlueprintHelperLibrary.GetBlackboard` (`AIBlueprintHelperLibrary.GetAIController` self)) "HasSeenPlayer" false)
  (`AudioComponent.StopDelayed` (`self.JoggerSound_1`) 0.2)
  (`AudioComponent.StopDelayed` (`self.JoggerSound_2`) 0.2)
  (`AudioComponent.StopDelayed` (`self.JoggerSound_3`) 0.2)
  (`AudioComponent.StopDelayed` (`self.JoggerSound_4`) 0.2))

(event `self.Box.OnComponentBeginOverlap`
  (params (OverlappedComponent :type "PrimitiveComponent Object Reference") (OtherActor :type "Actor Object Reference") (OtherComp :type "PrimitiveComponent Object Reference") (OtherBodyIndex :type Integer) (bFromSweep :type Boolean) (SweepResult :type "HitResult Structure (by ref)"))
  (bind (_returnvalue_roll _returnvalue_pitch _returnvalue_yaw) (`KismetMathLibrary.BreakRotator` (`SceneComponent.K2_GetComponentRotation` (`self.Box`))))
  (bind _asbp_player_character (cast `/Game/Characters/Wraith/BP_PlayerCharacter` OtherActor))
  (`|AIMoveTo` self (`SceneComponent.K2_GetComponentLocation` (`self.Box`)) null
    (:`then`
      (`CharacterMovementComponent.DisableMovement` (`Character.CharacterMovement` _asbp_player_character))
      (`self.K2_SetActorRotation` _asbp_player_character (`KismetMathLibrary.MakeRotator` _returnvalue_roll _returnvalue_pitch (+ _returnvalue_yaw 180.0)) false)
      (bind _returnvalue (`self.PlayAnimMontage` "/Game/Characters/Enemies/Draugr/AM_Draugr_Grab.AM_Draugr_Grab"))
      (`self.PlayAnimMontage` _asbp_player_character "/Game/Characters/Wraith/WraithAssets/AM_Wraith_GetGrabbed.AM_Wraith_GetGrabbed" 1.0 "None")
      (`KismetSystemLibrary.Delay` _returnvalue)
      (bind _asgm_bp_manager (cast `/Game/GameManager/GM_BP_Manager` (`GameplayStatics.GetGameMode`)))
      (`/Game/GameManager/GM_BP_Manager.Load Game` _asgm_bp_manager))))

(fn `HandlesHearing`
  (params (Player :type "Actor Object Reference") (Stimulus :type "AIStimulus Structure"))
  (bind _returnvalue (`GameplayStatics.GetPlayerCharacter` 0))
  (bind _joggersound_4 (`self.JoggerSound_4`))
  (bind _returnvalue_2 (`AIPerceptionSystem.GetSenseClassForStimulus` Stimulus))
  (if (== _returnvalue_2 "/Script/AIModule.AISense_Hearing")
    (bind _asplayer_character (cast `PlayerCharacter` _returnvalue))
    (if (== (`local.Player`) _returnvalue)
      (bind (_returnvalue_x _returnvalue_y) (`KismetMathLibrary.BreakVector` (`self.GetVelocity` _asplayer_character)))
      (if (or (>= 1.0 _returnvalue_x) (>= _returnvalue_y 1.0))
        (set `self.CoughtPlayer?` true)
        (`BlackboardComponent.SetValueAsBool` (`AIBlueprintHelperLibrary.GetBlackboard` (`AIBlueprintHelperLibrary.GetAIController` self)) "HasSeenPlayer" true)
        (`AudioComponent.Play` (`KismetArrayLibrary.Array_Random` (`|MakeArray` (`self.JoggerSound_1`) (`self.JoggerSound_2`) (`self.JoggerSound_3`))) 0.0)
        (if (not (`AudioComponent.IsPlaying` _joggersound_4))
          (`AudioComponent.Play` _joggersound_4 0.0))
        (else
          (return)))
      (else
        (return)))
    (else
      (return))))

(fn `HandlesSight`
  (params (Player :type "Actor Object Reference") (Stimulus :type "AIStimulus Structure"))
  (bind _outitem (`KismetArrayLibrary.Array_Random` (`|MakeArray` (`self.JoggerSound_1`) (`self.JoggerSound_2`) (`self.JoggerSound_3`))))
  (bind _returnvalue (`AIPerceptionSystem.GetSenseClassForStimulus` Stimulus))
  (if (== _returnvalue "/Script/AIModule.AISense_Sight")
    (if (== (`local.Player`) (`GameplayStatics.GetPlayerCharacter` 0))
      (set `self.CoughtPlayer?` true)
      (`BlackboardComponent.SetValueAsBool` (`AIBlueprintHelperLibrary.GetBlackboard` (`AIBlueprintHelperLibrary.GetAIController` self)) "HasSeenPlayer" true)
      (`AudioComponent.AdjustVolume` _outitem 0.0 0.3 "Linear")
      (`AudioComponent.Play` _outitem 0.0)
      (else
        (return)))
    (else
      (return))))

(fn `UserConstructionScript`)