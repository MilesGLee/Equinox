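; A point light actor that flickers by continually varying its intensity and attenuation radius.
; A looping timer picks a random target intensity and offsets the base Range up or down by a random intensity-range value scaled by RangeModifier.
; Tick lerps the light toward both targets with fixed alphas, radius more slowly, so smoothing depends on frame rate.
; The construction script applies the base Range as the initial radius.
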(event `Change Intensity`
  (if (`self.canChange`)
    (`self.FluctuateVariables`)))

(event `self.ReceiveBeginPlay`
  (set `self.canChange` true)
  (`KismetSystemLibrary.K2_SetTimerDelegate` (delegate `Change Intensity`) 0.2 true))

(event `self.ReceiveTick`
  (params (DeltaSeconds :type "Float (single-precision)"))
  (bind _pointlightcomponent (`self.PointLightComponent`))
  (`LightComponent.SetIntensity` _pointlightcomponent (`KismetMathLibrary.Lerp` (`LightComponentBase.Intensity` _pointlightcomponent) (`self.Desired Intensity`) 0.05))
  (`LocalLightComponent.SetAttenuationRadius` (`self.PointLightComponent`) (`KismetMathLibrary.Lerp` (`LocalLightComponent.AttenuationRadius` _pointlightcomponent) (`self.Desired Range`) 0.005)))

(fn `FluctuateVariables`
  (bind _range (`self.Range`))
  (bind _returnvalue (`KismetMathLibrary.RandomFloatInRange` (`self.Min Intensity`) (`self.Max Intensity`)))
  (bind _returnvalue_2 (* _returnvalue (`self.Range Modifier`)))
  (set `self.Desired Intensity` _returnvalue)
  (if (>= _returnvalue (/ (+ (`self.Max Intensity`) (`self.Min Intensity`)) 2.0))
    (set `self.Desired Range` (+ _range _returnvalue_2))
    (else
      (set `self.Desired Range` (- _range _returnvalue_2)))))

(fn `UserConstructionScript`
  (`LocalLightComponent.SetAttenuationRadius` (`self.PointLightComponent`) (`self.Range`)))