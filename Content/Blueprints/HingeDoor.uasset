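; Hinged door Blueprint that swings a static mesh between closed and opened yaw angles when interacted with, starting closed.
; An event bound to OnInteract toggles the closed state, only once if SingleUse is set.
; Tick eases the mesh's world rotation toward the target by a fixed-alpha shortest-path lerp, so swing speed depends on frame rate and the angles are absolute world yaw.
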(event `self.ReceiveBeginPlay`
  (set `self.isClosed` true)
  (add `self.OnInteract` (delegate `OnInteractEvent`)))

(event `self.ReceiveTick`
  (params (DeltaSeconds :type "Float (single-precision)"))
  (bind _staticmesh (`self.StaticMesh`))
  (if (`self.isClosed`)
    (set `self.angle` (`self.closedAngle`))
    (else
      (set `self.angle` (`self.openedAngle`))))
  (`SceneComponent.K2_SetWorldRotation` _staticmesh (`KismetMathLibrary.RLerp` (`SceneComponent.K2_GetComponentRotation` _staticmesh) (`KismetMathLibrary.MakeRotator` 0.0 0.0 (`self.angle`)) 0.05 true) false false))

(event `OnInteractEvent`
  (if (`self.singleUse`)
    (if (not (`self.used`))
      (set `self.used` true)
      (set `self.isClosed` (not (`self.isClosed`)) :!label _label))
    (else
      (goto _label))))

(fn `UserConstructionScript`)