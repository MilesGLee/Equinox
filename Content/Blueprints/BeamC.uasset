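; BeamC is an actor with a Niagara beam effect that switches on when the game mode reports a beacon state.
; The effect is deactivated on BeginPlay.
; Each tick it reads the BeconLoad3 flag from GM_BP_Manager and activates the Niagara component once when the flag is set, guarded by IsActivated.
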(event `self.ReceiveBeginPlay`
  (`ActorComponent.Deactivate` (`self.Niagara`)))

(event `self.ReceiveTick`
  (params (DeltaSeconds :type "Float (single-precision)"))
  (bind _asgm_bp_manager (cast `/Game/GameManager/GM_BP_Manager` (`GameplayStatics.GetGameMode`)))
  (if (`/Game/GameManager/GM_BP_Manager.BeconLoad3` _asgm_bp_manager)
    (if (not (`self.IsActivated`))
      (`ActorComponent.Activate` (`self.Niagara`) false)
      (set `self.IsActivated` true))))

(fn `UserConstructionScript`)