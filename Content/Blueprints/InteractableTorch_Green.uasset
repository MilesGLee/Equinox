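; Interactable torch, named as a green variant, with a Niagara effect and a light that starts lit with a fire burst.
; Each interaction toggles the on state and swaps the effect to smoke, which never returns to fire.
; SingleUse only records a Used flag and does not block later toggles.
; Tick drives the light's range from the Intensity variable while on, and zero while off.
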(event `self.ReceiveBeginPlay`
  (set `self.isOn` true)
  (add `self.OnInteract` (delegate `On Interact Event`))
  (`NiagaraComponent.SetAsset` (`self.Niagara`) "/Game/FX/Fire/NS_FireBurst.NS_FireBurst" true))

(event `On Interact Event`
  (if (`self.single use`)
    (if (not (`self.used`))
      (set `self.used` true)))
  (set `self.isOn` (not (`self.isOn`)))
  (`NiagaraComponent.SetAsset` (`self.Niagara`) "/Game/FX/Smoke/NS_SMoke.NS_SMoke" true))

(event `self.ReceiveTick`
  (params (DeltaSeconds :type "Float (single-precision)"))
  (if (`self.isOn`)
    (set `/Game/Blueprints/DetailedLight.Range` (`self.intensity`) (`self.light`))
    (else
      (set `/Game/Blueprints/DetailedLight.Range` 0.0 (`self.light`)))))

(fn `UserConstructionScript`)