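; Door01 is a sliding door actor that eases between a closed and an open position.
; At BeginPlay it stores its placed location as closed and an Arrow component's world location as open.
; Each Tick it lerps from its current location toward the target chosen by IsOpen, using a small fixed alpha for frame-rate-dependent ease-out without sweep.
; Nothing in this Blueprint's graphs sets IsOpen.
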(event `self.ReceiveBeginPlay`
  (set `self.ClosedPosition` (`self.K2_GetActorLocation`))
  (set `self.OpenPosition` (`SceneComponent.K2_GetComponentLocation` (`self.Arrow`))))

(event `self.ReceiveTick`
  (params (DeltaSeconds :type "Float (single-precision)"))
  (if (`self.IsOpen`)
    (`self.K2_SetActorLocation` (`KismetMathLibrary.VLerp` (`self.K2_GetActorLocation`) (`self.OpenPosition`) 0.01))
    (else
      (`self.K2_SetActorLocation` (`KismetMathLibrary.VLerp` (`self.K2_GetActorLocation`) (`self.ClosedPosition`) 0.01)))))

(fn `UserConstructionScript`)