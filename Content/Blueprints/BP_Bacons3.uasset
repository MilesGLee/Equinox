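; Third light beacon pedestal, which the player lights by interacting with it and which stays recorded as lit through the game mode's save.
; Interacting sets BeaconLoad3 on GM_BP_Manager and calls SaveGame.
; Shortly after BeginPlay, and on every Tick, a true flag swaps the mesh's crystal material and raises GemB emission in the MPC_Equinox parameter collection.
; The lit look is polled, so it is reapplied each frame.
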(event `self.ReceiveBeginPlay`
  (add `self.OnInteract` (delegate `LightBecon`))
  (bind _asgm_bp_manager (cast `/Game/GameManager/GM_BP_Manager` (`GameplayStatics.GetGameMode`)))
  (`KismetSystemLibrary.Delay` 0.3)
  (if (`/Game/GameManager/GM_BP_Manager.BeaconLoad3` _asgm_bp_manager)
    (`PrimitiveComponent.SetMaterial` (`self.StaticMesh`) 1 "/Game/Environments/Props/LightPedestal/MI_LightPedestal_Crystal2.MI_LightPedestal_Crystal2" :!label _label)
    (`KismetMaterialLibrary.SetScalarParameterValue` "/Game/Environments/Materials/MPC_Equinox.MPC_Equinox" "GemB Emiss" 35.0)))

(event `LightBecon`
  (bind _asgm_bp_manager (cast `/Game/GameManager/GM_BP_Manager` (`GameplayStatics.GetGameMode`)))
  (set `/Game/GameManager/GM_BP_Manager.BeaconLoad3` true _asgm_bp_manager)
  (`/Game/GameManager/GM_BP_Manager.Save Game` _asgm_bp_manager))

(event `self.ReceiveTick`
  (params (DeltaSeconds :type "Float (single-precision)"))
  (bind _asgm_bp_manager (cast `/Game/GameManager/GM_BP_Manager` (`GameplayStatics.GetGameMode`)))
  (if (`/Game/GameManager/GM_BP_Manager.BeaconLoad3` _asgm_bp_manager)
    (goto _label)))

(fn `UserConstructionScript`)