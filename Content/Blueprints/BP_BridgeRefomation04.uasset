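; Bridge actor that reforms when interacted with and lights its beacon crystal, with the state saved through the game mode.
; BeginPlay binds the interact event, caches the mesh's placed transform, then teleports it to the Arrow's displaced pose.
; Interaction sets LoadBridge4 on GM_BP_Manager and saves.
; While that flag is true, Tick eases the mesh back with a fixed-alpha, frame-rate-dependent lerp and swaps the beacon material after a short delay.
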(event `self.ReceiveBeginPlay`
  (bind _staticmesh (`self.StaticMesh`))
  (bind _asgm_bp_manager (cast `/Game/GameManager/GM_BP_Manager` (`GameplayStatics.GetGameMode`)))
  (add `self.OnInteract` (delegate `OnInteractEvent`))
  (set `self.BrigeTransform` (`SceneComponent.K2_GetComponentToWorld` _staticmesh))
  (`SceneComponent.K2_SetWorldTransform` _staticmesh (`SceneComponent.K2_GetComponentToWorld` (`self.Arrow`)) false true))

(event `OnInteractEvent`
  (set `/Game/GameManager/GM_BP_Manager.LoadBridge4` true (stale `self.ReceiveBeginPlay` _asgm_bp_manager))
  (`/Game/GameManager/GM_BP_Manager.Save Game` (stale `self.ReceiveBeginPlay` _asgm_bp_manager)))

(event `self.ReceiveTick`
  (params (DeltaSeconds :type "Float (single-precision)"))
  (bind _staticmesh (`self.StaticMesh`))
  (if (`/Game/GameManager/GM_BP_Manager.LoadBridge4` (stale `self.ReceiveBeginPlay` _asgm_bp_manager))
    (`SceneComponent.K2_SetWorldTransform` _staticmesh (`KismetMathLibrary.TLerp` (`SceneComponent.K2_GetComponentToWorld` _staticmesh) (`self.BrigeTransform`) 0.012) true false)
    (`KismetSystemLibrary.Delay` 0.2)
    (`PrimitiveComponent.SetMaterial` (`self.Becon`) 1 "/Game/Environments/Props/LightPedestal/MI_LightPedestal_Crystal3.MI_LightPedestal_Crystal3")))

(fn `UserConstructionScript`)