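; Interactable lever trigger that moves the graveyard bridge meshes and saves its activated state.
; On BeginPlay it records each mesh's starting location and an end location offset by Axis times Distance.
; Interacting sets the GraveyardBridge flag on GM_BP_Manager and saves the game.
; Tick reads that flag to lerp every mesh toward its start or end location, rotating the lever while active.
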(event `self.ReceiveBeginPlay`
  (add `self.OnInteract` (delegate `On Interact Event`))
  (bind _asgm_bp_manager (cast `/Game/GameManager/GM_BP_Manager` (`GameplayStatics.GetGameMode`)))
  (for _array_element (`self.Meshes`)
    (bind _returnvalue (`SceneComponent.K2_GetComponentLocation` (`StaticMeshActor.StaticMeshComponent` _array_element)))
    (`KismetArrayLibrary.Array_Add` (`self.Starting Locations`) _returnvalue)
    (`KismetArrayLibrary.Array_Add` (`self.Ending Locations`) (+ _returnvalue (* (`self.Axis`) (`self.Distance`))))))

(event `On Interact Event`
  (bind _output_get (set `/Game/GameManager/GM_BP_Manager.GraveyardBridge` true (stale `self.ReceiveBeginPlay` _asgm_bp_manager)))
  (`/Game/GameManager/GM_BP_Manager.Save Game` (stale `self.ReceiveBeginPlay` _asgm_bp_manager)))

(event `self.ReceiveTick`
  (params (DeltaSeconds :type "Float (single-precision)"))
  (for (_array_element _array_index) (`self.Meshes`)
    (if (not (stale `On Interact Event` _output_get))
      (`self.K2_SetActorLocation` _array_element (`KismetMathLibrary.VLerp` (`self.K2_GetActorLocation` _array_element) (`|GetArrayItem` (`self.Starting Locations`) _array_index) (`self.Speed`)) false false)
      (else
        (`self.K2_SetActorLocation` _array_element (`KismetMathLibrary.VLerp` (`self.K2_GetActorLocation` _array_element) (`|GetArrayItem` (`self.Ending Locations`) _array_index) (`self.Speed`)) false false)
        (`SceneComponent.K2_SetWorldRotation` (`self.lever`) (`KismetMathLibrary.Conv_VectorToRotator` (`KismetMathLibrary.VLerp` (-60.0 0.0 0.0) (`KismetMathLibrary.Conv_RotatorToVector` (`SceneComponent.K2_GetComponentRotation` (`self.lever`))) 0.02)) false false)))))

(fn `UserConstructionScript`)