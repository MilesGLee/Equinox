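; Door01_2 is a sliding door actor that opens while the game mode's BeaconLoad1 flag is set and closes otherwise.
; On BeginPlay it stores its own location as closed and an Arrow component's world location as open.
; Each Tick it casts the game mode to GM_BP_Manager and lerps its location toward the matching position by a fixed alpha, giving a frame-rate-dependent ease.
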(event `self.ReceiveBeginPlay`
  (set `self.ClosedPosition` (`self.K2_GetActorLocation`))
  (set `self.OpenPosition` (`SceneComponent.K2_GetComponentLocation` (`self.Arrow`))))

(event `self.ReceiveTick`
  (params (DeltaSeconds :type "Float (single-precision)"))
  (bind _asgm_bp_manager (cast `/Game/GameManager/GM_BP_Manager` (`GameplayStatics.GetGameMode`)))
  (if (`/Game/GameManager/GM_BP_Manager.BeaconLoad1` _asgm_bp_manager)
    (`self.K2_SetActorLocation` (`KismetMathLibrary.VLerp` (`self.K2_GetActorLocation`) (`self.OpenPosition`) 0.01))
    (else
      (`self.K2_SetActorLocation` (`KismetMathLibrary.VLerp` (`self.K2_GetActorLocation`) (`self.ClosedPosition`) 0.01)))))

(fn `UserConstructionScript`)