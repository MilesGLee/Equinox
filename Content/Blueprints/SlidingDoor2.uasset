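; Interactable sliding door that moves an array of mesh actors between their placed positions and an offset of Axis times Distance.
; BeginPlay caches both endpoints and binds the OnInteract event, which toggles IsOpen, only once if SingleUse is set.
; Tick lerps each actor from its current location using Speed as alpha, giving frame-rate-dependent easing.
; IsOpen true targets the starting positions, false the offset ones.
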(event `self.ReceiveBeginPlay`
  (add `self.OnInteract` (delegate `On Interact Event`))
  (for _array_element (`self.Meshes`)
    (bind _returnvalue (`SceneComponent.K2_GetComponentLocation` (`StaticMeshActor.StaticMeshComponent` _array_element)))
    (`KismetArrayLibrary.Array_Add` (`self.Starting Locations`) _returnvalue)
    (`KismetArrayLibrary.Array_Add` (`self.Ending Locations`) (+ _returnvalue (* (`self.Axis`) (`self.Distance`))))))

(event `On Interact Event`
  (if (`self.Single Use`)
    (if (not (`self.IsUsed`))
      (set `self.IsUsed` true)
      (set `self.IsOpen` (not (`self.IsOpen`)) :!label _label))
    (else
      (goto _label))))

(event `self.ReceiveTick`
  (params (DeltaSeconds :type "Float (single-precision)"))
  (for (_array_element _array_index) (`self.Meshes`)
    (if (`self.IsOpen`)
      (`self.K2_SetActorLocation` _array_element (`KismetMathLibrary.VLerp` (`self.K2_GetActorLocation` _array_element) (`|GetArrayItem` (`self.Starting Locations`) _array_index) (`self.Speed`)) false false)
      (else
        (`self.K2_SetActorLocation` _array_element (`KismetMathLibrary.VLerp` (`self.K2_GetActorLocation` _array_element) (`|GetArrayItem` (`self.Ending Locations`) _array_index) (`self.Speed`)) false false)))))

(fn `UserConstructionScript`)