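; Game manager that saves and restores progress in a single save slot: player transform, camera data, and bridge, beacon, door and graveyard bridge states.
; BeginPlay loads the save, teleports the player, copies states into its variables, applies camera data after short delays and re-saves, or creates a save if none exists.
; LoadGame restarts the level so BeginPlay reloads the save.
; RestartLevel deletes the save before restarting.
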(event `Save Game`
  ;[1 1 1] Save Game
  (bind _returnvalue (`GameplayStatics.LoadGameFromSlot` "Save1"))
  (bind _asplayer_character (cast `PlayerCharacter` (`GameplayStatics.GetPlayerCharacter` 0)))
  (bind _assave_game_bp (cast `/Game/GameManager/SaveGame_BP` _returnvalue))
  (bind _asmain_camera (cast `MainCamera` (`PlayerCharacter.PlayerCamera` _asplayer_character)))
  (set `/Game/GameManager/SaveGame_BP.LastSavedChrarTransform` (`self.GetTransform` _asplayer_character) _assave_game_bp)
  (set `/Game/GameManager/SaveGame_BP.CameraDataSave` (`MainCamera.CurrentCameraData` _asmain_camera) _assave_game_bp)
  (set `/Game/GameManager/SaveGame_BP.GraveYardBridgeSave` (`self.GraveyardBridge`) _assave_game_bp)
  (set `/Game/GameManager/SaveGame_BP.BlueAreaBrickDoorSave` (`self.BlueAreaBrickDoor`) _assave_game_bp)
  (set `/Game/GameManager/SaveGame_BP.BeconSave3` (`self.BeaconLoad3`) _assave_game_bp)
  (set `/Game/GameManager/SaveGame_BP.BeconSave1` (`self.BeaconLoad1`) _assave_game_bp)
  (set `/Game/GameManager/SaveGame_BP.BeconSave2` (`self.BeaconLoad2`) _assave_game_bp)
  (`|ExecutionSequence`
    (:`then_0`
      (set `/Game/GameManager/SaveGame_BP.BridgeSave1` (`self.LoadBridge1`) _assave_game_bp))
    (:`then_1`
      (set `/Game/GameManager/SaveGame_BP.BridgeSave2` (`self.LoadBridge2`) _assave_game_bp))
    (:`then_2`
      (set `/Game/GameManager/SaveGame_BP.BridgeSave3` (`self.LoadBridge3`) _assave_game_bp))
    (:`then_3`
      (set `/Game/GameManager/SaveGame_BP.BridgeSave4` (`self.LoadBridge4`) _assave_game_bp))
    (:`then_4`
      (set `/Game/GameManager/SaveGame_BP.BridgeSave5` (`self.LoadBridge5`) _assave_game_bp)))
  (`GameplayStatics.SaveGameToSlot` _assave_game_bp "Save1"))

(event `self.ReceiveBeginPlay`
  (bind _returnvalue (`GameplayStatics.DoesSaveGameExist` "Save1"))
  (if _returnvalue
    ;[1 1 1] Load Game Funtionality
    (bind _returnvalue_2 (`GameplayStatics.LoadGameFromSlot` "Save1"))
    (bind _assave_game_bp (cast `/Game/GameManager/SaveGame_BP` _returnvalue_2))
    (bind _asplayer_character (cast `PlayerCharacter` (`GameplayStatics.GetPlayerCharacter` 0)))
    (`self.K2_SetActorTransform` _asplayer_character (`/Game/GameManager/SaveGame_BP.LastSavedChrarTransform` _assave_game_bp) false true)
    (`KismetSystemLibrary.Delay` 0.2)
    (bind _asmain_camera (cast `MainCamera` (`PlayerCharacter.PlayerCamera` _asplayer_character)))
    (set `self.BlueAreaBrickDoor` (`/Game/GameManager/SaveGame_BP.BlueAreaBrickDoorSave` _assave_game_bp))
    (set `self.BeaconLoad1` (`/Game/GameManager/SaveGame_BP.BeconSave1` _assave_game_bp))
    (set `self.BeaconLoad2` (`/Game/GameManager/SaveGame_BP.BeconSave2` _assave_game_bp))
    (set `self.BeaconLoad3` (`/Game/GameManager/SaveGame_BP.BeconSave3` _assave_game_bp))
    (set `self.GraveyardBridge` (`/Game/GameManager/SaveGame_BP.GraveYardBridgeSave` _assave_game_bp))
    (`|ExecutionSequence`
      (:`then_0`
        (set `self.LoadBridge1` (`/Game/GameManager/SaveGame_BP.BridgeSave1` _assave_game_bp)))
      (:`then_1`
        (set `self.LoadBridge2` (`/Game/GameManager/SaveGame_BP.BridgeSave2` _assave_game_bp)))
      (:`then_2`
        (set `self.LoadBridge3` (`/Game/GameManager/SaveGame_BP.BridgeSave3` _assave_game_bp)))
      (:`then_3`
        (set `self.LoadBridge4` (`/Game/GameManager/SaveGame_BP.BridgeSave4` _assave_game_bp)))
      (:`then_4`
        (set `self.LoadBridge5` (`/Game/GameManager/SaveGame_BP.BridgeSave5` _assave_game_bp))))
    (`KismetSystemLibrary.Delay` 0.1)
    (`MainCamera.SetCameraData` _asmain_camera (`/Game/GameManager/SaveGame_BP.CameraDataSave` _assave_game_bp))
    (`self.Save Game`)
    (else
      ;[1 1 1] Creates save game
      (bind _returnvalue_3 (`GameplayStatics.CreateSaveGameObject` "/Game/GameManager/SaveGame_BP.SaveGame_BP_C"))
      (bind _asplayer_character_2 (cast `PlayerCharacter` (`GameplayStatics.GetPlayerCharacter` 0)))
      (set `/Game/GameManager/SaveGame_BP.LastSavedChrarTransform` (`self.GetTransform` _asplayer_character_2) _returnvalue_3)
      (`GameplayStatics.SaveGameToSlot` _returnvalue_3 "Save1"))))

(event `Load Game`
  ;[1 1 1] Load Game
  (`KismetSystemLibrary.ExecuteConsoleCommand` "RestartLevel" null))

(event `Restart Level`
  ;[1 1 1] Delete Save + Restart
  (`GameplayStatics.DeleteGameInSlot` "Save1")
  (`KismetSystemLibrary.ExecuteConsoleCommand` "RestartLevel" null))

(fn `UserConstructionScript`)